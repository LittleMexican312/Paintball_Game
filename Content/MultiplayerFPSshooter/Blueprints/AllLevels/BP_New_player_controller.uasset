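; Player controller for the multiplayer shooter that handles team setup, spawning and the player's UI.
; On BeginPlay it passes the game instance's team to the PlayerState, shows the HUD and requests a delayed, DoOnce-guarded spawn from the game mode.
; Events drive HUD widgets, death menu and scoreboard, while kill-log entries fan out to every controller through the game mode.
; Keys toggle the scoreboard, in-game menu and time-dilation debugging.
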(event Custom|Show%20HUD
  ;[0.1531 0.5493 1] show main hud
  (Utilities|IsValid (Variables|Default|GetHUD)
    (:Is%20Valid
      _)
    (:Is%20Not%20Valid
      (bind _returnvalue (UserInterface|CreateWidget "/Game/MultiplayerFPSshooter/widgets/Ingame/WBP_HUD.WBP_HUD_C" self))
      (Variables|Default|SetHUD _returnvalue)))
  (UserInterface|Viewport|AddtoViewport (Variables|Default|GetHUD) 0)
  (Input|SetInputModeGameOnly self))

(event Custom|damage%20indicator
  (params (Target :type Vector%20%28by%20ref%29))
  ;[1 1 1] hurt and damage indicator
  (Default|OnDamage (Variables|/Game/MultiplayerFPSshooter/widgets/Ingame/WBP_HUD.WBP_HUD_C|GetDamage_widget (Variables|Default|GetHUD)) Target))

(event Custom|PassCharacterInfoToServer
  (params (selected%20Team :type Integer))
  ;[1 0.7331 0] begin play
  (Variables|Default|SetSelected%20Team selected%20Team)
  (bind _asbp_playerstate (Utilities|Casting|CastToBP_playerstate (Variables|GetPlayerState)))
  (Default|SetTeam _asbp_playerstate (Variables|Default|GetSelected%20Team))
  (Networking|ForceNetUpdate)
  (Utilities|FlowControl|Delay 2.0)
  (CallFunction|SpawnthePlayer))

(event Custom|updatekilllog
  (params (Killer :type Text) (Victim :type Text) (headshot? :type Boolean) (IsAccidentDeath :type Boolean) (Killer%20team :type Integer) (weapon%20image :type Slate%20Brush%20Structure))
  ;[1 1 1] KILL LOG Process and handle incoming chat / Calls update chat on the Client
  (bind _asbp_third_person_game_mode (Utilities|Casting|CastToBP_ThirdPersonGameMode (Game|GetGameMode)))
  (for _array_element (Variables|/Game/MultiplayerFPSshooter/Blueprints/AllLevels/BP_ThirdPersonGameMode.BP_ThirdPersonGameMode_C|GetAllPlayerControllers _asbp_third_person_game_mode)
    (bind _asbp_new_player_controller (Utilities|Casting|CastToBP_New_player_controller _array_element))
    (CallFunction|UpdateKillLogClient _asbp_new_player_controller Killer Victim headshot? IsAccidentDeath Killer%20team weapon%20image)))

(event Custom|updateKillLogClient
  (params (Killer :type Text) (Victim :type Text) (headshot? :type Boolean) (IsAccidentDeath :type Boolean) (Killer%20team :type Integer) (weapon%20image :type Slate%20Brush%20Structure))
  ;[1 1 1] KILL LOG Process and handle incoming chat / Calls update chat on the Client
  (bind _returnvalue (UserInterface|CreateWidget "/Game/MultiplayerFPSshooter/widgets/Ingame/WBP_Kill_log_message.WBP_Kill_log_message_C" self Killer Victim headshot? IsAccidentDeath Killer%20team weapon%20image))
  (Default|EAddMessage (Variables|/Game/MultiplayerFPSshooter/widgets/Ingame/WBP_HUD.WBP_HUD_C|GetKill_log (Variables|Default|GetHUD)) _returnvalue))

(event Custom|hide%20HUD
  ;[1 1 1] hide hud
  (Widget|RemovefromParent (Variables|Default|GetHUD)))

(event Custom|killed%20player
  (params (Victim :type Text))
  ;[1 1 1] killed player widget
  (Default|KilledbyPalyerWidgetSetVisible (Variables|/Game/MultiplayerFPSshooter/widgets/Ingame/WBP_HUD.WBP_HUD_C|Getkilled_player (Variables|Default|GetHUD)) Victim))

(event Custom|show%20respawn%20widget
  (bind _ingamemenu (Variables|Default|Getingamemenu))
  ;[0.03692 0.3764 1] to show respawn menu when died
  (Utilities|IsValid (Variables|Default|GetDeathMenu)
    (:Is%20Valid
      (Widget|RemovefromParent (Variables|Default|GetDeathMenu)))
    (:Is%20Not%20Valid
      _))
  (bind _returnvalue (UserInterface|CreateWidget "/Game/MultiplayerFPSshooter/widgets/Ingame/WBP_DeathMenu.WBP_DeathMenu_C" self))
  (bind _output_get (Variables|Default|SetDeathMenu _returnvalue))
  (UserInterface|Viewport|AddtoViewport _output_get 0)
  (Variables|Default|SetbShowMouseCursor true)
  (Input|SetInputModeUIOnly self (Variables|Default|GetDeathMenu) "DoNotLock")
  (Utilities|IsValid _ingamemenu
    (:Is%20Valid
      (Widget|SetVisibility _ingamemenu "Hidden"))))

(event Custom|reload%20warn%20widget%20set%20anjim%20and%20sound%20PC
  ;[1 1 1] reload warn widget set in/visible PC
  (Default|ReloadWarnWidgetSetAnimandSound (Variables|/Game/MultiplayerFPSshooter/widgets/Ingame/WBP_HUD.WBP_HUD_C|Getreload_warn (Variables|Default|GetHUD))))

(event Custom|Spawn%20the%20player
  ;[1 1 1] spawn player
  (bind _asbp_third_person_game_mode (Utilities|Casting|CastToBP_ThirdPersonGameMode (Game|GetGameMode)))
  (Utilities|FlowControl|DoOnce false :!label _label
    (:Completed
      (Default|SpawnPlayer _asbp_third_person_game_mode self "/Game/MultiplayerFPSshooter/Blueprints/AllLevels/BP_ThirdPersonCharacter.BP_ThirdPersonCharacter_C" "/Game/MultiplayerFPSshooter/Blueprints/AllLevels/BP_assault_rifle_child.BP_assault_rifle_child_C" (Variables|GetPlayerState) (Variables|Default|GetSelected%20Team))
      (Utilities|FlowControl|RetriggerableDelay 5.0)
      (goto _label Reset))))

(event Custom|score%20widget
  (params (score :type Float%20%28single-precision%29) (score%20type :type Text))
  ;[1 1 1] SCORE widget
  (Default|SetScoreVisible (Variables|/Game/MultiplayerFPSshooter/widgets/Ingame/WBP_HUD.WBP_HUD_C|Getscore (Variables|Default|GetHUD)) score score%20type))

(event Custom|killed%20by%20player
  (params (Killer :type Text) (NewParam :type Actor%20Object%20Reference))
  ;[1 1 1] killed player widget
  (Default|KilledPalyerWidgetSetVisible (Variables|/Game/MultiplayerFPSshooter/widgets/Ingame/WBP_HUD.WBP_HUD_C|Getkilled_by_player (Variables|Default|GetHUD)) Killer NewParam))

(event Custom|hide%20scoreboard%20and%20visible%20respawn%20ui
  ;[1 1 1] hide scoreboard and visible respawn ui
  (Default|ESetScoreboardVisible (Variables|Default|GetHUD) false)
  (CallFunction|ShowRespawnWidgetClient))

(event Custom|reload%20time%20widget
  ;[1 1 1] reload time widget
  (Default|SetReloadTimeVisible (Variables|/Game/MultiplayerFPSshooter/widgets/Ingame/WBP_HUD.WBP_HUD_C|Getreload_time (Variables|Default|GetHUD))))

(event Custom|show%20respawn%20widget%20client
  (bind _ingamemenu (Variables|Default|Getingamemenu))
  ;[0.03692 0.3764 1] to show respawn menu when died
  (Utilities|IsValid (Variables|Default|GetDeathMenu)
    (:Is%20Valid
      (Widget|RemovefromParent (Variables|Default|GetDeathMenu)))
    (:Is%20Not%20Valid
      _))
  (bind _returnvalue (UserInterface|CreateWidget "/Game/MultiplayerFPSshooter/widgets/Ingame/WBP_DeathMenu.WBP_DeathMenu_C" self))
  (bind _output_get (Variables|Default|SetDeathMenu _returnvalue))
  (UserInterface|Viewport|AddtoViewport _output_get 0)
  (Variables|Default|SetbShowMouseCursor true)
  (Input|SetInputModeUIOnly self (Variables|Default|GetDeathMenu) "DoNotLock")
  (Utilities|IsValid _ingamemenu
    (:Is%20Valid
      (Widget|SetVisibility _ingamemenu "Hidden"))))

(event Custom|show%20scoreboard
  (params (end%20of%20match? :type Boolean))
  (bind _hud (Variables|Default|GetHUD))
  (bind _scoreboard_new (Variables|/Game/MultiplayerFPSshooter/widgets/Ingame/WBP_HUD.WBP_HUD_C|GetScoreBoard_new _hud))
  ;[0 1 0.4144] show scoreboard after end of match
  (Default|ESetScoreboardVisible _hud true)
  ;[1 1 1] set input mode ui only at end of the match
  (Input|SetInputModeUIOnly self _scoreboard_new "DoNotLock")
  (Variables|Default|SetbShowMouseCursor true)
  (if end%20of%20match?
    (Default|ShowXPandFinalStats _scoreboard_new)
    (else
      (Default|ShowRoundTroundTime _scoreboard_new))))

(event EventBeginPlay
  ;[1 0.7331 0] begin play
  (bind _asbp_game_instance (Utilities|Casting|CastToBP_GameInstance (Game|GetGameInstance)))
  (CallFunction|PassCharacterInfotoServer (Variables|/Game/MultiplayerFPSshooter/Blueprints/AllLevels/BP_GameInstance.BP_GameInstance_C|GetSelected%20Team _asbp_game_instance))
  (CallFunction|ShowHUD))

(event Input|KeyboardEvents|U
  (params (Key :type Key%20Structure :default "None"))
  ;[1 1 1] For animation debuging (grenade throwing)
  (:Pressed
    (Utilities|FlowControl|FlipFlop
      (:A
        (Utilities|Time|SetGlobalTimeDilation 0.07))
      (:B
        (Utilities|Time|SetGlobalTimeDilation 1.0)))))

(event Input|KeyboardEvents|O
  (params (Key :type Key%20Structure :default "None"))
  ;[1 1 1] For animation debuging (grenade throwing)
  (:Pressed
    (Utilities|FlowControl|FlipFlop
      (:A
        (Utilities|Time|SetGlobalTimeDilation 1e+01))
      (:B
        (Utilities|Time|SetGlobalTimeDilation 1.0)))))

(event Input|KeyboardEvents|Escape
  (params (Key :type Key%20Structure :default "None"))
  (bind _hud (Variables|Default|GetHUD))
  ;[0.7975 0.6348 1] show old ingame menu DONT DELETE! ITS FOR TESTING
  (:Pressed
    (bind _returnvalue (Game|GetCurrentLevelName true))
    (if (not (Utilities|Enum|Equal(Enum) _returnvalue "MainMenu"))
      (if (Widget|IsVisible (Variables|/Game/MultiplayerFPSshooter/widgets/Ingame/WBP_HUD.WBP_HUD_C|GetingameMenu _hud))
        (Default|IngameMenuOff _hud)
        (else
          (Default|IngameMenuon _hud))))))

(event Input|KeyboardEvents|P
  (params (Key :type Key%20Structure :default "None"))
  ;[1 1 1] For animation debuging (grenade throwing)
  (:Pressed
    (Utilities|FlowControl|FlipFlop
      (:A
        (Utilities|Time|SetGlobalTimeDilation 4e+02))
      (:B
        (Utilities|Time|SetGlobalTimeDilation 1.0)))))

(event Input|KeyboardEvents|Tab
  (params (Key :type Key%20Structure :default "None"))
  (bind _hud (Variables|Default|GetHUD))
  ;[1 1 1] scoreboard
  (:Pressed
    (Default|ESetScoreboardVisible _hud true))
  (:Released
    (Default|ESetScoreboardVisible _hud false)))

(event Input|KeyboardEvents|Backspace
  (params (Key :type Key%20Structure :default "None"))
  (bind _hud (Variables|Default|GetHUD))
  ;[0.7975 0.6348 1] show old ingame menu DONT DELETE! ITS FOR TESTING
  (:Pressed
    (bind _returnvalue (Game|GetCurrentLevelName true))
    (if (not (Utilities|Enum|Equal(Enum) _returnvalue "MainMenu"))
      (if (Widget|IsVisible (Variables|/Game/MultiplayerFPSshooter/widgets/Ingame/WBP_HUD.WBP_HUD_C|GetingameMenu _hud))
        (Default|IngameMenuOff _hud)
        (else
          (Default|IngameMenuon _hud))))))

(fn ConstructionScript)