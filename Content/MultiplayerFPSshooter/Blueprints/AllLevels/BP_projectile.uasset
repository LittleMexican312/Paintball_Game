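; BP_projectile is a multiplayer shooter projectile that triggers an X icon on the HUD when it hits a living character.
; On BeginPlay its collision ignores the owner and instigator while moving.
; On authority, a hit from a character-owned projectile calls XIconEvent, then destroys the actor.
; XIconEvent checks that the hit character is not dead, then signals the X icon widget through player controller 0's HUD.
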(event Custom|x%20icon%20event
  (params (Hit :type Hit%20Result%20Structure%20%28by%20ref%29))
  (bind _hitactor (Collision|BreakHitResult Hit))
  (bind _asbp_third_person_character (Utilities|Casting|CastToBP_ThirdPersonCharacter _hitactor))
  (Utilities|IsValid _asbp_third_person_character
    (:Is%20Valid
      (if (not (Variables|/Game/MultiplayerFPSshooter/Blueprints/AllLevels/BP_ThirdPersonCharacter.BP_ThirdPersonCharacter_C|GetIsDead? _asbp_third_person_character))
        (bind _asbp_new_player_controller (Utilities|Casting|CastToBP_New_player_controller (Game|GetPlayerController 0)))
        (Default|XIconEvent (Variables|/Game/MultiplayerFPSshooter/widgets/Ingame/WBP_HUD.WBP_HUD_C|GetWBP_X_icon (Variables|/Game/MultiplayerFPSshooter/Blueprints/AllLevels/BP_New_player_controller.BP_New_player_controller_C|GetHUD _asbp_new_player_controller)))))))

(event Collision|EventActorBeginOverlap
  (params (OtherActor :type Actor%20Object%20Reference)))

(event EventTick
  (params (DeltaSeconds :type Float%20%28single-precision%29)))

(event Collision|EventHit
  (params (MyComp :type Primitive%20Component%20Object%20Reference) (Other :type Actor%20Object%20Reference) (OtherComp :type Primitive%20Component%20Object%20Reference) (bSelfMoved :type Boolean) (HitLocation :type Vector :default "0, 0, 0") (HitNormal :type Vector :default "0, 0, 0") (NormalImpulse :type Vector :default "0, 0, 0") (Hit :type Hit%20Result%20Structure%20%28by%20ref%29))
  ;[1 1 1] OnEventHit
  (Networking|SwitchHasAuthority
    (:Authority
      (Utilities|IsValid (.AsBP%20Third%20Person%20Character (Utilities|Casting|CastToBP_ThirdPersonCharacter (Components|GetOwner)))
        (:Is%20Valid
          (CallFunction|XIconEvent Hit)
          (Actor|DestroyActor))))))

(event EventBeginPlay
  ;[1 1 1] event begin play
  (Collision|IgnoreActorwhenMoving (Variables|Default|GetProjectileCollision) (Components|GetOwner) true)
  (Collision|IgnoreActorwhenMoving (Variables|Default|GetProjectileCollision) (Game|GetInstigator) true))

(fn ConstructionScript)