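; Base weapon for the multiplayer FPS, handling server-side firing, ammo and timed reloads.
; Single, auto and burst modes feed a two-stage sphere trace, from camera to aim point, then from muzzle to that point.
; Hits apply point damage scaled by random criticals and physical material, and spawn a projectile.
; Multicast events play sounds and impact effects, while owning-client events add recoil, crosshair kick and floating damage text.
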(event Custom|dynamic%20crosshair%20and%20floating%20damage%20on%20clinet
  ;[1 1 1] dynamic crosshair
  (bind _asbp_new_player_controller (Utilities|Casting|CastToBP_New_player_controller (Pawn|GetController (Variables|Default|Getplayer%20character%20Ref))))
  (Default|ShootEvent (Variables|/Game/MultiplayerFPSshooter/widgets/Ingame/WBP_HUD.WBP_HUD_C|GetCrossHair_ (Variables|/Game/MultiplayerFPSshooter/Blueprints/AllLevels/BP_New_player_controller.BP_New_player_controller_C|GetHUD _asbp_new_player_controller))))

(event Custom|Multicast_ReloadSound
  (bind _reload_time (Variables|Default|GetReload%20time))
  ;[1 1 1] Reload Weapon
  (Utilities|FlowControl|Delay 0.3)
  (Audio|SpawnSoundAttached (Variables|sounds|GetReload%20begin%20Sound) (Variables|Default|GetSK_WeaponMesh) "None" "0, 0, 0" "0, 0, 0" "KeepRelativeOffset" false 1.0 (* _reload_time 2.0) 0.0 0 0) ; start reload sound
  (Utilities|FlowControl|Delay (- _reload_time 0.8))
  (Audio|SpawnSoundAttached (Variables|sounds|GetReload%20end%20Sound) (Variables|Default|GetSK_WeaponMesh) "None" "0, 0, 0" "0, 0, 0" "KeepRelativeOffset" false 1.0 1.0 0.0 0 0) ; end reload sound
)

(event Custom|recoil%20run%20owning%20client
  (bind _player_character_ref (Variables|Default|Getplayer%20character%20Ref))
  (bind _recoil (Variables|Default|GetRecoil))
  (bind _player_character_ref_2 (Variables|Default|Getplayer%20character%20Ref))
  (bind _recoil_2 (Variables|Default|GetRecoil))
  (bind _player_character_ref_3 (Variables|Default|Getplayer%20character%20Ref))
  (bind _recoil_3 (Variables|Default|GetRecoil))
  (bind _returnvalue (/ _recoil_2 8e+01))
  (bind _returnvalue_2 (/ _recoil 2e+02))
  (bind _istakingcover (Variables|/Game/MultiplayerFPSshooter/Blueprints/AllLevels/BP_ThirdPersonCharacter.BP_ThirdPersonCharacter_C|GetIsTakingCover _player_character_ref))
  (bind _returnvalue_3 (select _istakingcover 4e+02 2e+02))
  (bind _returnvalue_4 (/ _recoil_3 _returnvalue_3))
  (bind _returnvalue_5 (* _returnvalue_4 -1.0))
  ;[1 1 1] recoil
  (Camera|PlayWorldCameraShake "/Game/MultiplayerFPSshooter/Blueprints/AllLevels/BP_RecoilShakeAuto.BP_RecoilShakeAuto_C" (Transformation|GetWorldLocation (Variables|/Game/MultiplayerFPSshooter/Blueprints/AllLevels/BP_ThirdPersonCharacter.BP_ThirdPersonCharacter_C|GetCamera (Variables|Default|Getplayer%20character%20Ref))) 6e+01 1.2e+02)
  (Utilities|FlowControl|Sequence
    (:then_0
      (Utilities|FlowControl|Delay 0.05)
      ;;[1 1 1] for all gunrifle
      (Pawn|Input|AddControllerPitchInput _player_character_ref_3 (Math|Random|RandomFloatinRange _returnvalue_5 _returnvalue_5)) ; pitch
      ;;[1 1 1] for smooth pitch upward
      (Variables|/Game/MultiplayerFPSshooter/Blueprints/AllLevels/BP_ThirdPersonCharacter.BP_ThirdPersonCharacter_C|Setpitchrep _player_character_ref_2 (+ (Variables|/Game/MultiplayerFPSshooter/Blueprints/AllLevels/BP_ThirdPersonCharacter.BP_ThirdPersonCharacter_C|Getpitchrep _player_character_ref_2) _returnvalue))
      (Variables|/Game/MultiplayerFPSshooter/Blueprints/AllLevels/BP_ThirdPersonCharacter.BP_ThirdPersonCharacter_C|Setpitchnotrep _player_character_ref_2 (+ (Variables|/Game/MultiplayerFPSshooter/Blueprints/AllLevels/BP_ThirdPersonCharacter.BP_ThirdPersonCharacter_C|Getpitchnotrep _player_character_ref_2) _returnvalue)))
    (:then_1
      (Utilities|FlowControl|Delay 0.05)
      (Pawn|Input|AddControllerYawInput _player_character_ref_3 (Math|Random|RandomFloatinRange (* _returnvalue_2 -1.0) _returnvalue_2)) ; Yaw
    )))

(event Custom|SRV_ShootReleased
  (bind _player_character_ref (Variables|Default|Getplayer%20character%20Ref))
  (bind _isaiming_ (Variables|/Game/MultiplayerFPSshooter/Blueprints/AllLevels/BP_ThirdPersonCharacter.BP_ThirdPersonCharacter_C|GetIsAiming? _player_character_ref))
  (bind _aimcamera (Variables|/Game/MultiplayerFPSshooter/Blueprints/AllLevels/BP_ThirdPersonCharacter.BP_ThirdPersonCharacter_C|GetaimCamera _player_character_ref))
  (bind _camera (Variables|/Game/MultiplayerFPSshooter/Blueprints/AllLevels/BP_ThirdPersonCharacter.BP_ThirdPersonCharacter_C|GetCamera _player_character_ref))
  (bind _returnvalue (select _isaiming_ _aimcamera _camera))
  ;[0.8572 1 0] shoot beginning from player character BP
  (Utilities|AutoFireMode) ; enters at InputPin
)

(event Custom|spawn%20effects%20and%20ammo%20count
  (Variables|donotset|SetIsCooldownActive? true)
  (Variables|donotset|SetIsAutoFire? true)
  (CallFunction|MulticastFireWeaponFX)
  (CallFunction|DecrementAmmo)
  ;[1 1 1] single/multifire rate cooldown
  (Utilities|FlowControl|Delay (/ 6e+01 (Variables|Default|GetSingle/multiFireRate)))
  (Variables|donotset|SetIsCooldownActive? false))

(event Custom|ROS_LineTraceShot
  (params (trace%20Start :type Vector) (trace%20Orientation :type Rotator))
  (bind (_hitresult _hit) (CallFunction|WeaponSphereTrace trace%20Start trace%20Orientation))
  (Variables|Default|Sethit%20actor (.HitActor (Collision|BreakHitResult _hitresult)))
  (Utilities|FlowControl|Sequence
    (:then_0
      (Game|Damage|ApplyPointDamage (Variables|Default|Gethit%20actor) (* (Variables|Default|GetBase%20Damage) (Variables|Default|Getcritical%20damage%20scale) (select (Utilities|IsValid (.PhysMat (Collision|BreakHitResult _hitresult))) (Variables|/Script/PhysicsCore.PhysicalMaterial|GetDestructibleDamageThresholdScale (.PhysMat (Collision|BreakHitResult _hitresult))) 1.0)) (.Location (Collision|BreakHitResult _hitresult)) _hitresult (Game|GetInstigatorController) (Components|GetOwner))
      (Utilities|IsValid (Game|GetInstigator)
        (:Is%20Valid
          (CallFunction|FloatingDamageOwningClient _hitresult (Utilities|Text|ToText(Float) (* (Variables|Default|GetBase%20Damage) (Variables|Default|Getcritical%20damage%20scale) (select (Utilities|IsValid (.PhysMat (Collision|BreakHitResult _hitresult))) (Variables|/Script/PhysicsCore.PhysicalMaterial|GetDestructibleDamageThresholdScale (.PhysMat (Collision|BreakHitResult _hitresult))) 1.0)) "HalfToEven") (Variables|donotset|GetCritical%20shoot?) (.HitBoneName (Collision|BreakHitResult _hitresult)))
          (CallFunction|FSSpawnProjectile _hitresult _hit) ; CONTAINS PROJECTILE SPAWN AND CRITICAL SYSTEM
          (CallFunction|EffectsMulticast _hitresult)
          (Utilities|FlowControl|Sequence
            (:then_0
              (CallFunction|SpawnEffectsandAmmoCount))
            (:then_1
              ;[1 0.0426 0] single/multifire rate cooldown ITS FOR changing fire mode
              (Utilities|FlowControl|Delay (Variables|Default|GetSingle/multiFireRate))
              (Variables|donotset|SetIsCooldownActive? false))
            (:then_2
              (CallFunction|RecoilRunOwningClient)
              (CallFunction|DynamicCrosshairandFloatingDamageonClinet))))))
    (:then_1
      ;[0.9472 1 0.8746] 2. critical chance
      (bind _output_get (Variables|donotset|SetCritical%20shoot? (<= (Math|Random|RandomIntegerinRangefromStream 0 100 (Variables|donotset|Getrandom%20stream)) (Variables|Default|GetCriticalMultiplier))))
      (if _output_get
        (Variables|Default|Setcritical%20damage%20scale 2.0)
        (else
          (Variables|Default|Setcritical%20damage%20scale 1.0))))))

(event Custom|SRV_ShootPressed
  (bind _player_character_ref (Variables|Default|Getplayer%20character%20Ref))
  (bind _isaiming_ (Variables|/Game/MultiplayerFPSshooter/Blueprints/AllLevels/BP_ThirdPersonCharacter.BP_ThirdPersonCharacter_C|GetIsAiming? _player_character_ref))
  (bind _aimcamera (Variables|/Game/MultiplayerFPSshooter/Blueprints/AllLevels/BP_ThirdPersonCharacter.BP_ThirdPersonCharacter_C|GetaimCamera _player_character_ref))
  (bind _camera (Variables|/Game/MultiplayerFPSshooter/Blueprints/AllLevels/BP_ThirdPersonCharacter.BP_ThirdPersonCharacter_C|GetCamera _player_character_ref))
  (bind _returnvalue (select _isaiming_ _aimcamera _camera))
  ;[0.8572 1 0] shoot beginning from player character BP
  ;[1 1 1] to be sure its on server
  (Networking|SwitchHasAuthority
    (:Authority
      (switch Utilities|FlowControl|Switch|SwitchonEN_Firing_mode (Variables|Default|GetFiringMode)
        (:NewEnumerator0
          (Utilities|SingleFireMode
            (:true
              _)))
        (:NewEnumerator1
          (Utilities|AutoFireMode
            (:then_0
              _)))
        (:NewEnumerator2
          (Utilities|BurstFireMode
            (:then_0
              _))))
      ;[1 1 1] Stop Weapon Fire If Ammo Is = To Zero
      (if (not (<= (Variables|donotset|GetCurrentAmmoInClip) 0))
        (Utilities|FlowControl|Sequence
          (:then_0
            (CallFunction|ROSLineTraceShot (Transformation|GetWorldLocation _returnvalue) (Transformation|GetWorldRotation _returnvalue)))
          (:then_1
            (CallFunction|SetReloadWarn)))))))

(event Custom|Server_OnWeaponReload
  ;[1 1 1] Reload Weapon
  (Variables|Default|SetReload%20started true)
  (CallFunction|MulticastReloadSound)
  (Utilities|FlowControl|Delay (Variables|Default|GetReload%20time))
  (CallFunction|ReloadAddAmmo)
  (Variables|Default|SetReload%20started false))

(event Custom|effects%20multicast
  (params (Hit :type Hit%20Result%20Structure%20%28by%20ref%29))
  (bind (_bblockinghit _binitialoverlap _time _distance _location _impactpoint _normal _impactnormal _physmat _hitactor) (Collision|BreakHitResult Hit))
  ;[1 1 1] Effects
  ;;[1 1 1] filter to not show effects on characters
  (Utilities|IsValid (.AsBP%20Third%20Person%20Character (Utilities|Casting|CastToBP_ThirdPersonCharacter _hitactor))
    (:Is%20Not%20Valid
      (Audio|PlaySoundatLocation (Variables|sounds|GetDefaultBulletImpactSound) _location "0, 0, 0" 1.0 1.0 0.0 0 0 0)
      (Effects|SpawnEmitteratLocation 0 _location)
      (Rendering|Decal|SpawnDecalatLocation "/Game/MultiplayerFPSshooter/materials/M_bullet_hole.M_bullet_hole" "15.000000,15.000000,15.000000" _location (Math|Rotator|MakeRotfromXZ _impactnormal (Transformation|GetActorLocation)) 1e+01))))

(event Custom|Multicast_FireWeaponFX
  ;[1 1 1] MultiFire Weapon FX
  (CallFunction|FireWeaponFX))

(event Custom|floating%20damage%20owning%20client
  (params (Hit :type Hit%20Result%20Structure%20%28by%20ref%29) (dmg :type Text) (crt? :type Boolean) (InSocketName :type Name))
  (bind _hitactor (Collision|BreakHitResult Hit))
  (bind _asbp_third_person_character (Utilities|Casting|CastToBP_ThirdPersonCharacter _hitactor))
  ;[1 0.07388 0] spawn float damage actor
  (Utilities|IsValid _asbp_third_person_character
    (:Is%20Valid
      (if (not (Variables|/Game/MultiplayerFPSshooter/Blueprints/AllLevels/BP_ThirdPersonCharacter.BP_ThirdPersonCharacter_C|GetIsDead? _asbp_third_person_character)) ; dont spawn float damage if the victim is already dead
        (Variables|Default|Setmesh%20for%20floating%20damage (Variables|/Script/Engine.Character|GetMesh _asbp_third_person_character))
        (Game|SpawnActorfromClass "/Game/MultiplayerFPSshooter/Blueprints/AllLevels/BP_Floating_damage_text.BP_Floating_damage_text_C" (Math|Transform|MakeTransform (Transformation|GetSocketLocation (Variables|Default|Getmesh%20for%20floating%20damage) InSocketName) "0, 0, 0" "1,1,1") "AlwaysSpawn" 0 (Utilities|Name|Equal(Name) InSocketName "head") crt? dmg 0)))))

(event EventIESetOwnerCharacter
  (params (Character :type Character%20Object%20Reference))
  ;[1 1 1] set player char ref
  (bind _asbp_third_person_character (Utilities|Casting|CastToBP_ThirdPersonCharacter Character))
  (Variables|Default|Setplayer%20character%20Ref _asbp_third_person_character) ; 3p_player char. ref
)

(event EventBeginPlay
  ;[0 1 0.07414] set default ammo
  (Variables|donotset|SetCurrentMaxAmmo (Variables|Default|GetMaxAmmo))
  (Variables|donotset|SetCurrentAmmoInClip (Variables|Default|GetMaxAmmoClipSize))
  ;[1 0.2732 0] set the basic spread counting the accuracy,auto weapons must be more
  (Variables|donotset|Setspread (* (- 1e+02 (Variables|Default|GetAccuracy)) 4e+02)))

(event EventTick
  (params (DeltaSeconds :type Float%20%28single-precision%29)))

(event Collision|EventActorBeginOverlap
  (params (OtherActor :type Actor%20Object%20Reference)))

(event EventIEShootPressed
  ;[0.8572 1 0] shoot beginning from player character BP
  (CallFunction|SRVShootPressed))

(event EventIEShootReleased
  ;[0.8572 1 0] shoot beginning from player character BP
  (CallFunction|SRVShootReleased))

(fn ConstructionScript)

(fn WeaponSphereTrace
  (params (A :type Vector) (InRot :type Rotator))
  (bind _player_character_ref (Variables|Default|Getplayer%20character%20Ref))
  (bind _array (Utilities|Array|MakeArray _player_character_ref))
  (Utilities|IsValid (Variables|Default|Getplayer%20character%20Ref)
    (:Is%20Valid
      (bind (_outhit _returnvalue) (Collision|SphereTraceByChannel A (Utilities|AddRandomSpread (+ A (* (Math|Vector|GetForwardVector InRot) (Variables|donotset|GetSphereTraceRange)))) (Variables|donotset|GetSphereTraceRadius) "TraceTypeQuery1" false _array "None" true "(R=0.000000,G=0.267520,B=1.000000,A=1.000000)"))
      (bind (_outhit_2 _returnvalue_2) (Collision|SphereTraceByChannel (Transformation|GetSocketLocation (Variables|Default|GetSK_WeaponMesh) (Variables|Default|GetMuzzleSocketName)) (Math|Vector|SelectVector (.ImpactPoint (Collision|BreakHitResult _outhit)) (.TraceEnd (Collision|BreakHitResult _outhit)) _returnvalue) (Variables|donotset|GetSphereTraceRadius) "TraceTypeQuery1" true _array "None"))
      (return _outhit_2 _returnvalue_2))))

(fn FSSpawnProjectile
  (params (Hit :type Hit%20Result%20Structure%20%28by%20ref%29) (A :type Boolean))
  (bind (_bblockinghit _binitialoverlap _time _distance _location _impactpoint _normal _impactnormal _physmat _hitactor _hitcomponent _hitbonename _hititem _faceindex _tracestart _traceend) (Collision|BreakHitResult Hit))
  (bind _player_character_ref (Variables|Default|Getplayer%20character%20Ref))
  (Networking|SwitchHasAuthority
    (:Authority
      ;[1 1 1] to wont be able to shoot
      (if (and A (not (Variables|/Game/MultiplayerFPSshooter/Blueprints/AllLevels/BP_ThirdPersonCharacter.BP_ThirdPersonCharacter_C|GetIsDead? _player_character_ref)))
        ;[1 1 1] spawn bullets projectile
        (Game|SpawnActorfromClass "/Game/MultiplayerFPSshooter/Blueprints/AllLevels/BP_projectile.BP_projectile_C" (Math|Transform|MakeTransform (Transformation|GetSocketLocation (Variables|BP_Baseweapon_C|GetSK_WeaponMesh (Variables|/Game/MultiplayerFPSshooter/Blueprints/AllLevels/BP_ThirdPersonCharacter.BP_ThirdPersonCharacter_C|GetBPCurrentWeaponRef _player_character_ref)) "aim") (Math|Rotator|FindLookatRotation (Transformation|GetSocketLocation (Variables|Default|GetSK_WeaponMesh) (Variables|Default|GetMuzzleSocketName)) (Math|Vector|SelectVector _impactpoint _traceend false))) "AlwaysSpawn" (Components|GetOwner) false _hitbonename (Game|GetInstigator))))))

(fn FireWeaponFX
  (Audio|SpawnSoundAttached (Variables|sounds|GetSingleFireSound) (Variables|Default|GetSK_WeaponMesh) (Variables|Default|GetMuzzleSocketName) "0, 0, 0" "0, 0, 0" "KeepRelativeOffset" false (Variables|Default|Getweapon%20volume) 1.0 0.0 0 0))

(fn DecrementAmmo
  (Variables|donotset|SetCurrentAmmoInClip (Math|Integer|Clamp(Integer) (- (Variables|donotset|GetCurrentAmmoInClip) 1) 0 (Variables|Default|GetMaxAmmoClipSize))))

(fn ReloadAddAmmo
  (Networking|SwitchHasAuthority
    (:Authority
      (Variables|donotset|SetAmmoNeededForReload (- (Variables|Default|GetMaxAmmoClipSize) (Variables|donotset|GetCurrentAmmoInClip)))
      (if (<= (Variables|donotset|GetCurrentMaxAmmo) (Variables|donotset|GetAmmoNeededForReload))
        (Variables|donotset|SetCurrentAmmoInClip (+ (Variables|donotset|GetCurrentAmmoInClip) (Variables|donotset|GetCurrentMaxAmmo)))
        (Variables|donotset|SetCurrentMaxAmmo 0)
        (else
          (Variables|donotset|SetCurrentMaxAmmo (- (Variables|donotset|GetCurrentMaxAmmo) (Variables|donotset|GetAmmoNeededForReload)))
          (Variables|donotset|SetCurrentAmmoInClip (Variables|Default|GetMaxAmmoClipSize)))))))

(fn SetReloadWarn
  (if (== (Math|Conversions|ToFloat(Integer) (Variables|donotset|GetCurrentAmmoInClip)) (Math|Conversions|ToFloat(Integer) (/ (* (Variables|Default|GetMaxAmmoClipSize) 35) 100)))
    (bind _asbp_new_player_controller (Utilities|Casting|CastToBP_New_player_controller (Game|GetPlayerController 0)))
    ;[1 1 1] visibility is in WBP_HUD bind
    (Default|ReloadWarnWidgetSetAnjimandSoundPC _asbp_new_player_controller)))

(fn IFGetDamage)