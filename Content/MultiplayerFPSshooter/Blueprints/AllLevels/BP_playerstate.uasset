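; Player state for the multiplayer FPS that tracks a player's kills, deaths, score and selected team.
; Simple functions increment kills and deaths, add to the score, and assign the team.
; Score and team changes run only with authority, while the kill and death counters have no authority check.
; Team assignment also prints red or blue for the chosen team.
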(event EventBeginPlay)

(event EventTick
  (params (DeltaSeconds :type Float%20%28single-precision%29)))

(fn ConstructionScript)

(fn AddKill
  (Math|Integer|IncrementInt (Variables|Default|GetKills)))

(fn AddDeaths
  (Math|Integer|IncrementInt (Variables|Default|GetDeaths)))

(fn AddScore
  (params (A :type Integer))
  (Networking|SwitchHasAuthority
    (:Authority
      (Variables|Default|Setown%20score (+ A (Variables|Default|Getown%20score))))))

(fn SetTeam
  (params (selected%20team :type Integer))
  (Networking|SwitchHasAuthority
    (:Authority
      (bind _output_get (Variables|Default|Setselected%20team selected%20team))
      (switch int _output_get
        (:0
          (Development|PrintString "red"))
        (:1
          (Development|PrintString "blue"))))))