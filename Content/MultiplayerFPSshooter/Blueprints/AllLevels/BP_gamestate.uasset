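; Game State for the multiplayer FPS that runs the match clock and tracks team scores and map, server and mode info from the Game Instance.
; A looping authority timer decrements match time unless paused, and on expiry decides the winning team and notifies the Game Mode.
; A DoOnce-gated second-round path pauses play, counts down and resets the clock.
; Team scores are summed from each PlayerState on the server.
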(event Custom|Score%20Collecting
  ;[1 1 1] team score
  (Networking|SwitchHasAuthority
    (:Authority
      (Variables|Default|SetBlue%20Team%20Score 0)
      (Variables|Default|SetRed%20Team%20score 0)
      (for _array_element (Variables|Default|GetPlayerArray)
        (bind _asbp_playerstate (Utilities|Casting|CastToBP_playerstate _array_element))
        (if (== (Variables|/Game/MultiplayerFPSshooter/Blueprints/AllLevels/BP_playerstate.BP_playerstate_C|Getselected%20team _asbp_playerstate) 0)
          (Variables|Default|SetRed%20Team%20score (+ (Variables|/Game/MultiplayerFPSshooter/Blueprints/AllLevels/BP_playerstate.BP_playerstate_C|Getown%20score _asbp_playerstate) (Variables|Default|GetRed%20Team%20score)))
          (elif (== (Variables|/Game/MultiplayerFPSshooter/Blueprints/AllLevels/BP_playerstate.BP_playerstate_C|Getselected%20team _asbp_playerstate) 1)
            (Variables|Default|SetBlue%20Team%20Score (+ (Variables|/Game/MultiplayerFPSshooter/Blueprints/AllLevels/BP_playerstate.BP_playerstate_C|Getown%20score _asbp_playerstate) (Variables|Default|GetBlue%20Team%20Score)))))))))

(event Custom|start%20count%20time
  ;[1 0.02291 0] Begin Play. Start  match timer
  (Networking|SwitchHasAuthority
    (:Authority
      (bind _returnvalue (Utilities|Time|SetTimerbyFunctionName 0 "IE_RoundTimeCountDown" 1.0 true))
      (Variables|Default|SetRoundTimer _returnvalue))))

(event Custom|match%20end%20sound%20and%20score%20collecting
  ;[1 1 1] match end sound and score collecting
  (Utilities|FlowControl|DoOnce false
    (:Completed
      (if (> (Variables|Default|GetRed%20Team%20score) (Variables|Default|GetBlue%20Team%20Score))
        (Variables|Default|SetRed%20team%20won? true)
        (Development|PrintString "red team won")
        (else
          (Variables|Default|SetRed%20team%20won? false)
          (Development|PrintString "blue team won"))))))

(event Custom|start%20second%20round
  ;[0 1 0.8943] Match time Countdown. Finish match when time expired
  (Variables|Default|SetPause true)
  (if (== (Variables|Default|GetRounds) 1) ; round or match end?
    ;;[0.5162 1 0] first round done
    (Utilities|FlowControl|Sequence
      (:then_0
        (if (not (<= (Variables|Default|Getround%20begin%20time) 0))
          (Utilities|FlowControl|DoOnce false
            (:Completed
              (Utilities|Time|SetTimerbyFunctionName 0 "end round time" 1.0 true)))))
      (:then_1
        (Utilities|FlowControl|DoOnce false
          (:Completed
            (if (Networking|IsServer)
              ;;;[1 1 1] put something if you want to have 2 rounds
              ;;; whis would be after 1st round is ended
              (Development|PrintString "Hello"))))))
    (else
      ;;[0 0.2185 1] match is over
      (Utilities|FlowControl|DoOnce false
        (:Completed
          (CallFunction|MatchEndSoundandScoreCollecting)
          ;;;[1 1 1] match time is over
          (CallFunction|IFTimeisover true)
          (Default|Round/warmup/matchFinished (stale Custom|IE_RoundTimeCountDown _asbp_third_person_game_mode) true))))))

(event Custom|IE_RoundTimeCountDown
  ;[0 1 0.8943] Match time Countdown. Finish match when time expired
  (Utilities|FlowControl|Sequence
    (:then_0
      (if (Variables|Default|GetPause)
        (Development|PrintString "paused game")
        (elif (== (Variables|Default|GetMatch%20temp%20time) 0)
          (if (== (Variables|Default|GetRounds) 1) ; round or match end?
            ;;[0.5162 1 0] first round done
            (Utilities|FlowControl|Sequence
              (:then_0
                (if (not (<= (Variables|Default|Getround%20begin%20time) 0))
                  (Utilities|FlowControl|DoOnce false
                    (:Completed
                      (Utilities|Time|SetTimerbyFunctionName 0 "end round time" 1.0 true)))))
              (:then_1
                (Utilities|FlowControl|DoOnce false
                  (:Completed
                    (if (Networking|IsServer)
                      ;;;[1 1 1] put something if you want to have 2 rounds
                      ;;; whis would be after 1st round is ended
                      (Development|PrintString "Hello"))))))
            (else
              ;;[0 0.2185 1] match is over
              (Utilities|FlowControl|DoOnce false
                (:Completed
                  (CallFunction|MatchEndSoundandScoreCollecting)
                  ;;;[1 1 1] match time is over
                  (CallFunction|IFTimeisover true)
                  (Default|Round/warmup/matchFinished (stale _asbp_third_person_game_mode) true)))))
          (else
            (bind _asbp_third_person_game_mode (Utilities|Casting|CastToBP_ThirdPersonGameMode (Game|GetGameMode)))
            ;;[1 1 1] match time counting
            (if (not (Variables|/Game/MultiplayerFPSshooter/Blueprints/AllLevels/BP_ThirdPersonGameMode.BP_ThirdPersonGameMode_C|Gettime%20is%20over? _asbp_third_person_game_mode))
              (Math|Integer|DecrementInt (Variables|Default|GetMatch%20temp%20time)
                (:%20%20
                  (Math|Integer|DecrementInt (Variables|Default|GetmaxTime)))))))))
    (:then_1
      ;;[1 1 1] count match time
      (Math|Integer|IncrementInt (Variables|Default|Getwhole%20match%20time)))))

(event Custom|end%20round%20time
  (bind _round_begin_time (Variables|Default|Getround%20begin%20time))
  ;[0 1 0.8943] Match time Countdown. Finish match when time expired
  (if (<= _round_begin_time 0)
    (Utilities|FlowControl|DoOnce false
      (:Completed
        (Variables|Default|SetPause false)
        (Variables|Default|SetRounds 2)
        (CallFunction|IFInitgametime)
        (Audio|PlaySound2D 0 0.2 1.0 0.0 0 0)))
    (else
      (Math|Integer|DecrementInt _round_begin_time))))

(event EventBeginPlay
  ;[1 0.02291 0] Begin Play. Start  match timer
  (bind _asbp_game_instance (Utilities|Casting|CastToBP_GameInstance (Game|GetGameInstance)))
  (Variables|Default|SetMainGI _asbp_game_instance)
  (Variables|Default|SetRounds 0)
  (Variables|Default|SetMapName (Variables|/Game/MultiplayerFPSshooter/Blueprints/AllLevels/BP_GameInstance.BP_GameInstance_C|GetMapName (Variables|Default|GetMainGI)))
  (Variables|Default|SetServerName (Utilities|String|ToString(Text) (Variables|/Game/MultiplayerFPSshooter/Blueprints/AllLevels/BP_GameInstance.BP_GameInstance_C|GetServerName (Variables|Default|GetMainGI))))
  (Variables|Default|SetGameModeId (Variables|/Game/MultiplayerFPSshooter/Blueprints/AllLevels/BP_GameInstance.BP_GameInstance_C|GetGameModeId (Variables|Default|GetMainGI))))

(event EventTick
  (params (DeltaSeconds :type Float%20%28single-precision%29)))

(fn ConstructionScript)

(fn DeathTimer
  ;[1 1 1] CountDown Timer
  (if (not (and (<= (Variables|Default|GetDeathSeconds) 0) (<= (Variables|Default|GetDeathMinutes) 0)))
    (Variables|Default|SetDeathSeconds (- (Variables|Default|GetDeathSeconds) 1))
    (if (< (Variables|Default|GetDeathSeconds) 0)
      (Variables|Default|SetDeathSeconds (+ 10 (Variables|Default|GetDeathSeconds))))))

(fn IFTimeisover
  (params (end%20of%20match? :type Boolean))
  (Utilities|Time|PauseTimerbyHandle (Variables|Default|GetRoundTimer))
  (if (Networking|IsServer)
    ;[1 1 1] from gm
    (bind _asbp_third_person_game_mode (Utilities|Casting|CastToBP_ThirdPersonGameMode (Game|GetGameMode)))
    (Default|MatchEnd _asbp_third_person_game_mode end%20of%20match?)
    (return)))

(fn IFInitgametime
  (Utilities|FlowControl|Sequence
    (:then_0
      (Variables|Default|SetMatch%20temp%20time (* (Variables|/Game/MultiplayerFPSshooter/Blueprints/AllLevels/BP_GameInstance.BP_GameInstance_C|GetGameTime (Variables|Default|GetMainGI)) 60)) ; Original 600
    )
    (:then_1
      (return))))