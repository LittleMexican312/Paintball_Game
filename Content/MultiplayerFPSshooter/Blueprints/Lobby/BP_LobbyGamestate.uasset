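; Lobby game state for a multiplayer FPS that tracks player counts for the red team, the blue team and the lobby total.
; One function raises or lowers the red or blue count from a team index and a logout flag.
; A second function adjusts the total from a boolean, and both skip decrements at zero.
; The event graph and construction script hold no logic.
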(event EventBeginPlay)

(event EventTick
  (params (DeltaSeconds :type Float%20%28single-precision%29)))

(fn ConstructionScript)

(fn FSUpdateLobbyPlayers
  (params (OnLogoutLocal1 :type Boolean) (TeamLocal1 :type Integer))
  (LocalVariables|SetOnLogoutLocal OnLogoutLocal1)
  (LocalVariables|SetTeamLocal TeamLocal1)
  (switch int (LocalVariables|GetTeamLocal)
    (:0
      (if (LocalVariables|GetOnLogoutLocal)
        (if (!= (Variables|Default|GetLobbyRedPlayers) 0)
          (Variables|Default|SetLobbyRedPlayers (- (Variables|Default|GetLobbyRedPlayers) 1))
          (return))
        (else
          (Variables|Default|SetLobbyRedPlayers (+ (Variables|Default|GetLobbyRedPlayers) 1))
          (return))))
    (:1
      (if (LocalVariables|GetOnLogoutLocal)
        (if (!= (Variables|Default|GetLobbyBluePlayers) 0)
          (Variables|Default|SetLobbyBluePlayers (- (Variables|Default|GetLobbyBluePlayers) 1))
          (return))
        (else
          (Variables|Default|SetLobbyBluePlayers (+ (Variables|Default|GetLobbyBluePlayers) 1))
          (return))))))

(fn FSUpdateCurrentPlayers
  (params (Condition :type Boolean))
  (if Condition
    (if (!= (Variables|Default|GetTotalCurrentPlayers) 0)
      (Variables|Default|SetTotalCurrentPlayers (- (Variables|Default|GetTotalCurrentPlayers) 1)))
    (else
      (Variables|Default|SetTotalCurrentPlayers (+ (Variables|Default|GetTotalCurrentPlayers) 1)))))